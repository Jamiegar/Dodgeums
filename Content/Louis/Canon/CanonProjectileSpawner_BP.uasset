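; Cannon spawner that launches projectiles from its own transform at random intervals, starting on BeginPlay.
; Each Fire call re-sets its own looping timer with a new random delay of a few seconds, then spawns one of three projectile classes.
; Selection uses two chained random rolls, so the three types are not equally likely.
; Spawn yaw passes through the RandomRotation helper, intended to add slight angular spread.
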(event `self.ReceiveBeginPlay`
  (`self.Fire`))

(event `Fire`
  (bind _returnvalue (`self.GetTransform`))
  (bind _returnvalue_2 (`self.GetTransform`))
  (bind _returnvalue_3 (`self.GetTransform`))
  (`KismetSystemLibrary.K2_SetTimerDelegate` (delegate `Fire`) (`KismetMathLibrary.RandomFloatInRange` 1.0 3.0) true)
  (if (== (`KismetMathLibrary.RandomIntegerInRange` 1 3) 1)
    (`|SpawnActorFromClass` "/Game/Louis/Canon/Projectile1_BP.Projectile1_BP_C" (`KismetMathLibrary.MakeTransform` (.location _returnvalue) (`KismetMathLibrary.MakeRotator` (.roll (.rotation _returnvalue)) (.pitch (.rotation _returnvalue)) (`self.RandomRotation` (.yaw (.rotation _returnvalue)))) (.scale _returnvalue)) "Undefined" "OverrideRootScale" null null)
    (elif (== (`KismetMathLibrary.RandomIntegerInRange` 1 3) 2)
      (`|SpawnActorFromClass` "/Game/Louis/Canon/Projectile2_BP.Projectile2_BP_C" (`KismetMathLibrary.MakeTransform` (.location _returnvalue_2) (`KismetMathLibrary.MakeRotator` (.roll (.rotation _returnvalue_2)) (.pitch (.rotation _returnvalue_2)) (`self.RandomRotation` (.yaw (.rotation _returnvalue_2)))) (.scale _returnvalue_2)) "Undefined" "OverrideRootScale" null null)
      (else
        (`|SpawnActorFromClass` "/Game/Louis/Canon/Projectile3_BP.Projectile3_BP_C" (`KismetMathLibrary.MakeTransform` (.location _returnvalue_3) (`KismetMathLibrary.MakeRotator` (.roll (.rotation _returnvalue_3)) (.pitch (.rotation _returnvalue_3)) (`self.RandomRotation` (.yaw (.rotation _returnvalue_3)))) (.scale _returnvalue_3)) "Undefined" "OverrideRootScale" null null)))))

(fn `UserConstructionScript`)