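; BP_DeathVolume is a box kill volume whose extent is set from a BoxExtent variable in the construction script.
; On overlap it queries the actor with GetAICharacterMessage.
; If that succeeds, it calls CanEnd on BP_GameMode and gives the actor a short life span.
; Any other actor receives a DeathMessage call instead.
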(event `self.Box.OnComponentBeginOverlap`
  (params (OverlappedComponent :type "PrimitiveComponent Object Reference") (OtherActor :type "Actor Object Reference") (OtherComp :type "PrimitiveComponent Object Reference") (OtherBodyIndex :type Integer) (bFromSweep :type Boolean) (SweepResult :type "HitResult Structure (by ref)"))
  (bind (_aicharacter _succcess) (message `/Game/Tech/Interfaces/BPI_AI.GetAICharacter` OtherActor))
  (if _succcess
    (bind _asbp_game_mode (cast `/Game/Tech/Game/BP_GameMode` (`GameplayStatics.GetGameMode`)))
    (`/Game/Tech/Game/BP_GameMode.CanEnd?` _asbp_game_mode)
    (`self.SetLifeSpan` OtherActor 10.0)
    (else
      (message `/Game/Tech/Interfaces/BPI_Death.Death` OtherActor))))

(fn `UserConstructionScript`
  (`BoxComponent.SetBoxExtent` (`self.Box`) (`self.BoxExtent`) true))