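; Cannon spawner actor that repeatedly fires BP_ProjectileBase projectiles from its own transform, starting on BeginPlay.
; Each shot keeps the actor's roll, pitch and scale, and passes yaw through RandomRotation for a random spread.
; Fire activates the NSProjectileImpact effect, then clears and re-arms a non-looping timer with a random delay, so shot intervals vary.
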(event `self.ReceiveBeginPlay`
  (`self.Fire`)
  (`self.SetTimer`))

(event `SetTimer`
  (bind _returnvalue (`KismetSystemLibrary.K2_SetTimerDelegate` (delegate `Fire`) (`KismetMathLibrary.RandomFloatInRange` 1.0 2.0)))
  (set `self.Timer` _returnvalue))

(event `Fire`
  (bind (_returnvalue_location _returnvalue_rotation _returnvalue_scale) (`KismetMathLibrary.BreakTransform` (`self.GetTransform`)))
  (`|SpawnActorFromClass` "/Game/Tech/LevelAssets/Canon/BP_ProjectileBase.BP_ProjectileBase_C" (`KismetMathLibrary.MakeTransform` _returnvalue_location (`KismetMathLibrary.MakeRotator` (.roll _returnvalue_rotation) (.pitch _returnvalue_rotation) (`self.RandomRotation` (.yaw _returnvalue_rotation))) _returnvalue_scale) "Undefined" "OverrideRootScale" null null)
  (`ActorComponent.Activate` (`self.NS_ProjectileImpact`) false)
  (`KismetSystemLibrary.K2_ClearAndInvalidateTimerHandle` (`self.Timer`))
  (`self.SetTimer`))

(fn `UserConstructionScript`)