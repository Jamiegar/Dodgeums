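; BP_ProjectileBase is a base projectile Blueprint, filed with the Canon level assets, that varies its look per instance and expires on its own.
; The construction script gives the Sphere component a random mesh from StaticMeshArray and a random relative rotation.
; BeginPlay applies the LifeSpan variable as the actor's lifespan; the graphs hold no movement or hit logic.
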(event `self.ReceiveBeginPlay`
  (`self.SetLifeSpan` (`self.LifeSpan`)))

(fn `UserConstructionScript`
  (`StaticMeshComponent.SetStaticMesh` (`self.Sphere`) (`KismetArrayLibrary.Array_Random` (`self.StaticMeshArray`)))
  (`SceneComponent.K2_SetRelativeRotation` (`self.Sphere`) (`KismetMathLibrary.RandomRotator` false) false false))