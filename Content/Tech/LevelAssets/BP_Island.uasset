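; BP_Island is a level actor whose island mesh gets pushed by projectile hits and can ease back to level rotation.
; ProjectileHit applies an impulse at the impact point, along and scaled by the hit's trace vector.
; LerpBackToOrgin opens a gate on Tick that interpolates actor rotation toward zero, closing once zero is reached.
; Only rotation is restored; location is left untouched.
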(event `/Game/Tech/Interfaces/BPI_Damageable.ProjectileHit`
  (params (HitLocation :type "HitResult Structure"))
  (bind (_bblockinghit _binitialoverlap _time _distance _location _impactpoint _normal _impactnormal _physmat _hitactor _hitcomponent _hitbonename _bonename _hititem _elementindex _faceindex _tracestart _traceend) (`GameplayStatics.BreakHitResult` HitLocation))
  (`PrimitiveComponent.AddImpulseAtLocation` (`self.IslandMesh`) (* (- _traceend _tracestart) 250.0) _impactpoint "None"))

(event `self.ReceiveTick`
  (params (DeltaSeconds :type "Float (single-precision)"))
  (bind _returnvalue (`KismetMathLibrary.RInterpTo` (`self.K2_GetActorRotation`) (struct) DeltaSeconds 0.5))
  (`/Engine/EditorBlueprintResources/StandardMacros.Gate` true :!label _label
    (:`Exit`
      (`self.K2_SetActorRotation` _returnvalue)
      (if (== _returnvalue (struct))
        (goto _label :!via `Close`)))))

(event `LerpBackToOrgin`
  (goto _label :!via `Open`))

(fn `UserConstructionScript`)