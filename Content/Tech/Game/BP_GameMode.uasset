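; Game mode that runs the match flow from main menu to win or lose screen.
; BeginGame initialises the player and spawned AI controllers at BP_CustomSpawn points, hands each a game mode reference, then starts the cannon spawner and music.
; A separately triggered one-second looping timer counts down to Fail, while repeated CanEnd? calls raise an AI counter until the win.
; Either ending pauses the game, shows its widget and fades the music.
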(event `self.ReceiveBeginPlay`
  (bind _returnvalue (`GameplayStatics.GetPlayerController` 0))
  (bind _returnvalue_2 (`|CreateWidget` "/Game/Tech/UI/MainMenu/MainMenu.MainMenu_C"))
  (`UserWidget.AddToViewport` _returnvalue_2 0)
  (`WidgetBlueprintLibrary.SetInputMode_UIOnlyEx` _returnvalue null)
  (set `PlayerController.bShowMouseCursor` true _returnvalue))

(event `BeginGame`
  (set `PlayerController.bShowMouseCursor` false (`GameplayStatics.GetPlayerController` 0))
  (bind _outactors (`GameplayStatics.GetAllActorsOfClass` "/Game/Tech/Game/BP_CustomSpawn.BP_CustomSpawn_C"))
  ;[1 1 1] redo for mutliple player characters
  (set `self.CustomSpawns` _outactors)
  (bind _asbp_player_controller (cast `/Game/Tech/Game/Character/BP_PlayerController` (`GameplayStatics.GetPlayerController` 0)))
  (bind _output_get (set `self.PlayerController` _asbp_player_controller))
  (set `/Game/Tech/Game/Character/BP_PlayerController.GameMode` self _output_get)
  (`/Game/Tech/Game/Character/BP_PlayerController.Init` _output_get (`self.GetTransform` (`|GetArrayItem` (`self.CustomSpawns`))))
  (`KismetArrayLibrary.Array_Remove` (`self.CustomSpawns`))
  (for _index (range 3)
    (bind _returnvalue (`|SpawnActorFromClass` "/Game/Tech/AI/BP_AIController.BP_AIController_C" (`self.GetTransform` (`|GetArrayItem` (`self.CustomSpawns`) _index)) "Undefined" "OverrideRootScale" null null))
    (`KismetArrayLibrary.Array_AddUnique` (`self.AI Controllers`) _returnvalue))
  (for _array_element (`self.AI Controllers`)
    (set `/Game/Tech/AI/BP_AIController.GameMode` self _array_element)
    (`/Game/Tech/AI/BP_AIController.Init` _array_element))
  (bind _outactors_2 (`GameplayStatics.GetAllActorsOfClass` "/Game/Tech/LevelAssets/Canon/CanonProjectileSpawner_BP.CanonProjectileSpawner_BP_C"))
  (bind _output (`|GetArrayItem` _outactors_2))
  (`/Game/Tech/LevelAssets/Canon/CanonProjectileSpawner_BP.Fire` _output)
  (`/Game/Tech/LevelAssets/Canon/CanonProjectileSpawner_BP.SetTimer` _output)
  (bind _returnvalue_2 (`GameplayStatics.SpawnSound2D` "/Game/Tech/BackgroundMusic_S.BackgroundMusic_S" 1.0 1.0 0.0 null))
  (set `self.Sound` _returnvalue_2))

(event `5Min Timer`
  (`KismetSystemLibrary.K2_SetTimerDelegate` (delegate `StartTimer`) 1.0 true -1.0))

(event `StartTimer`
  (if (> (`self.Timer`) 0)
    (set `self.Timer` (- (`self.Timer`) 1))
    (if (== (`self.Timer`) 0)
      (`self.Fail`))))

(event `Fail`
  (bind _returnvalue (`GameplayStatics.GetPlayerController` 0))
  (`WidgetLayoutLibrary.RemoveAllWidgets`)
  (bind _returnvalue_2 (`|CreateWidget` "/Game/Tech/UI/Lose.Lose_C"))
  (`UserWidget.AddToViewport` _returnvalue_2 0)
  (`GameplayStatics.SetGamePaused` true)
  (`WidgetBlueprintLibrary.SetInputMode_UIOnlyEx` _returnvalue null)
  (set `PlayerController.bShowMouseCursor` true _returnvalue)
  (`AudioComponent.FadeOut` (`self.Sound`) 1.0 0.0 "Linear"))

(event `CanEnd?`
  (bind _returnvalue (`GameplayStatics.GetPlayerController` 0))
  (bind _result (`/Engine/EditorBlueprintResources/StandardMacros.IncrementInt` (`self.AICounter`))
    (:`  `
      (if (> _result 2)
        (`WidgetLayoutLibrary.RemoveAllWidgets`)
        (bind _returnvalue_2 (`|CreateWidget` "/Game/Tech/UI/Winner.Winner_C"))
        (`UserWidget.AddToViewport` _returnvalue_2 0)
        (`GameplayStatics.SetGamePaused` true)
        (`WidgetBlueprintLibrary.SetInputMode_UIOnlyEx` _returnvalue null)
        (set `PlayerController.bShowMouseCursor` true _returnvalue)
        (`AudioComponent.FadeOut` (`self.Sound`) 1.0 0.0 "Linear")))))

(fn `UserConstructionScript`)